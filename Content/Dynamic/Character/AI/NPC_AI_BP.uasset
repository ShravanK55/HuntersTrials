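; AI controller for guard NPCs that starts the GuardBehaviour behavior tree on the PatrolData blackboard at BeginPlay.
; Perception writes any sensed actor lacking the "Enemy" tag to the Enemy key and makes the controlled GameCharacter aim.
; Other perception updates clear that key but leave aiming on.
; Tick sets the character's ShouldShoot to whether the controller has a valid focus actor, which this Blueprint never sets itself.
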(event `self.ReceiveBeginPlay`
  (bind _blackboardcomponent (`self.UseBlackboard` "/Game/Dynamic/Character/AI/PatrolData.PatrolData"))
  (set `self.BlackboardComponent` _blackboardcomponent)
  (`self.RunBehaviorTree` "/Game/Dynamic/Character/AI/GuardBehaviour.GuardBehaviour"))

(event `self.AIPerception.OnTargetPerceptionUpdated`
  (params (Actor :type "Actor Object Reference") (Stimulus :type "AIStimulus Structure"))
  (bind _returnvalue (`KismetStringLibrary.Conv_StringToName` "Enemy"))
  (bind _blackboardcomponent (`self.BlackboardComponent`))
  (if (and (not (`self.ActorHasTag` Actor "Enemy")) (`.bSuccessfullySensed` (break `AIStimulus` Stimulus)))
    (`BlackboardComponent.SetValueAsObject` _blackboardcomponent _returnvalue Actor)
    (bind _asgame_character (cast `/Game/Dynamic/Character/Behaviour/GameCharacter` (`self.K2_GetPawn`)))
    (set `/Game/Dynamic/Character/Behaviour/GameCharacter.ShouldAim` true _asgame_character)
    (else
      (`BlackboardComponent.ClearValue` _blackboardcomponent _returnvalue))))

(event `self.ReceiveTick`
  (params (DeltaSeconds :type "Float (single-precision)"))
  (bind _asgame_character (cast `/Game/Dynamic/Character/Behaviour/GameCharacter` (`self.K2_GetPawn`)))
  (set `/Game/Dynamic/Character/Behaviour/GameCharacter.ShouldShoot` (`KismetSystemLibrary.IsValid` (`self.GetFocusActor`)) _asgame_character))

(fn `UserConstructionScript`)