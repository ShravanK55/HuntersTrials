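; NPC AI controller that drives a guard's behavior and tracks the actor it perceives as a target.
; On BeginPlay it initializes the PatrolData blackboard and runs the GuardBehaviour behavior tree.
; AI perception updates write sensed actors without the "Enemy" tag to the blackboard's Enemy key.
; Any other update, a lost stimulus or a tagged actor, clears that key.
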(event `self.ReceiveBeginPlay`
  (bind _blackboardcomponent (`self.UseBlackboard` "/Game/Dynamic/NPC/AI/PatrolData.PatrolData"))
  (set `self.BlackboardComponent` _blackboardcomponent)
  (`self.RunBehaviorTree` "/Game/Dynamic/NPC/AI/GuardBehaviour.GuardBehaviour"))

(event `self.AIPerception.OnTargetPerceptionUpdated`
  (params (Actor :type "Actor Object Reference") (Stimulus :type "AIStimulus Structure"))
  (bind _returnvalue (`KismetStringLibrary.Conv_StringToName` "Enemy"))
  (bind _blackboardcomponent (`self.BlackboardComponent`))
  (if (and (not (`self.ActorHasTag` Actor "Enemy")) (`.bSuccessfullySensed` (break `AIStimulus` Stimulus)))
    (`BlackboardComponent.SetValueAsObject` _blackboardcomponent _returnvalue Actor)
    (else
      (`BlackboardComponent.ClearValue` _blackboardcomponent _returnvalue))))

(fn `UserConstructionScript`)